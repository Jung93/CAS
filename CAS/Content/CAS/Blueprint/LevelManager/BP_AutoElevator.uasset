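; BP_AutoElevator is an elevator actor that automatically shuttles up and down between its starting location and a point a set Z offset away.
; BeginPlay caches both endpoints.
; Tick moves the actor at constant speed with VInterpToConstant, using the TargetReached flag to choose direction.
; On arrival at either end, a Delay pauses it briefly before the flag flips and it heads back.
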(event EventBeginPlay
  (bind _self self)
  (bind _returnvalue (Transformation|GetActorLocation _self))
  (Variables|Default|SetInitLocation _returnvalue)
  (Variables|Default|SetTargetLocation (+ _returnvalue (Math|Vector|MakeVector 0.0 0.0 (Variables|Default|GetOffSet)))))

(event Collision|EventActorBeginOverlap
  (params (OtherActor :type Actor%20Object%20Reference)))

(event EventTick
  (params (DeltaSeconds :type Float%20%28single-precision%29))
  (bind _self self)
  (bind _targetlocation (Variables|Default|GetTargetLocation))
  (bind _initlocation (Variables|Default|GetInitLocation))
  (bind _returnvalue (Transformation|GetActorLocation _self))
  (bind _returnvalue_2 (Transformation|GetActorLocation _self))
  (bind _returnvalue_3 (Math|Interpolation|VInterptoConstant _returnvalue_2 _initlocation DeltaSeconds 5e+02))
  (bind _returnvalue_4 (Math|Interpolation|VInterptoConstant _returnvalue _targetlocation DeltaSeconds 5e+02))
  (bind _returnvalue_5 (Utilities|Operators|EqualEqual _returnvalue_4 _targetlocation 0.0))
  (bind _returnvalue_6 (Utilities|Operators|NotEqual(!=) _returnvalue_3 _initlocation 0.0))
  (if (Variables|Default|GetTargetReached)
    (if _returnvalue_6
      _
      (else
        (Utilities|FlowControl|Delay 2.0)))
    (Variables|Default|SetTargetReached _returnvalue_6)
    (Transformation|SetActorLocation _returnvalue_3 false false)
    (else
      (if _returnvalue_5
        (Utilities|FlowControl|Delay 2.0))
      (Variables|Default|SetTargetReached _returnvalue_5)
      (Transformation|SetActorLocation _returnvalue_4 false false))))

(fn ConstructionScript)