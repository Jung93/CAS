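; BP_Brazier_01_TEST is a brazier actor that lights up once the puzzle is solved.
; On BeginPlay it deactivates its fire effect and zeroes two point lights.
; Every Tick it casts the game instance to CAS_GameInstance and polls IsPuzzleClear, re-activating the fire without reset and restoring both light intensities while that returns true.
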(event EventBeginPlay
  (Components|Activation|Deactivate (Variables|Default|GetP_Fire))
  (Rendering|Components|Light|SetIntensity (Variables|Default|GetPointLight) 0.0)
  (Rendering|Components|Light|SetIntensity (Variables|Default|GetPointLight1) 0.0))

(event Collision|EventActorBeginOverlap
  (params (OtherActor :type Actor%20Object%20Reference)))

(event EventTick
  (params (DeltaSeconds :type Float%20%28single-precision%29))
  (bind _ascas_game_instance (Utilities|Casting|CastToCAS_GameInstance (Game|GetGameInstance)))
  (bind _returnvalue (Class|CASGameInstance|IsPuzzleClear _ascas_game_instance))
  (if _returnvalue
    (Components|Activation|Activate (Variables|Default|GetP_Fire) false)
    (Rendering|Components|Light|SetIntensity (Variables|Default|GetPointLight) 9e+02)
    (Rendering|Components|Light|SetIntensity (Variables|Default|GetPointLight1) 1e+03)))

(fn ConstructionScript)