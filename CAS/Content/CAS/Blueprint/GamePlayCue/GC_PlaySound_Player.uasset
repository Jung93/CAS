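; Gameplay Cue for CAS_Player that plays a player sound effect when executed.
; OnExecute checks the PlayerState's ability system tags in priority order for fire breath, super speed, a test attack (round kick sound) and damage taken.
; The matching sound plays at world origin rather than at the player.
; All but the hit sound also report a noise event at the player's location, instigated by the player.
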(fn OnExecute
  (params (MyTarget :type Actor%20Object%20Reference) (Parameters :type Gameplay%20Cue%20Parameters%20Structure%20%28by%20ref%29))
  (bind _ascas_player (Utilities|Casting|CastToCAS_Player MyTarget))
  (LocalVariables|SetOwnerPlayer _ascas_player)
  (if (GameplayTags|HasMatchingGameplayTag (Ability|GetAbilitySystemComponent (Variables|/Script/Engine.Pawn|GetPlayerState _ascas_player)) "(TagName=\"Effect.Attack.FireBreath\")")
    (Audio|PlaySoundatLocation 0 "/Game/CAS/Resource/Sound/sound_FireBreath.sound_FireBreath" "0, 0, 0" "0, 0, 0" 1.0 1.0 0.0 0 0 0 0)
    (Class|AISenseHearing|ReportNoiseEvent 0 (Transformation|GetActorLocation (LocalVariables|GetOwnerPlayer)) 1.0 (LocalVariables|GetOwnerPlayer) 1e+03 "" :!label _label)
    (return false)
    (elif (GameplayTags|HasMatchingGameplayTag (Ability|GetAbilitySystemComponent (Variables|/Script/Engine.Pawn|GetPlayerState _ascas_player)) "(TagName=\"Effect.Move.SuperSpeed\")")
      (Audio|PlaySoundatLocation 0 "/Game/CAS/Resource/Sound/sound_SuperSpeed.sound_SuperSpeed" "0, 0, 0" "0, 0, 0" 1.0 1.0 0.0 0 0 0 0)
      (goto _label)
      (elif (GameplayTags|HasMatchingGameplayTag (Ability|GetAbilitySystemComponent (Variables|/Script/Engine.Pawn|GetPlayerState _ascas_player)) "(TagName=\"Effect.Attack.TEST\")")
        (Audio|PlaySoundatLocation 0 "/Game/CAS/Resource/Sound/sound_RoundKick.sound_RoundKick" "0, 0, 0" "0, 0, 0" 1.0 1.0 0.0 0 0 0 0)
        (goto _label)
        (elif (GameplayTags|HasMatchingGameplayTag (Ability|GetAbilitySystemComponent (Variables|/Script/Engine.Pawn|GetPlayerState _ascas_player)) "(TagName=\"State.TakeDamage\")")
          (Audio|PlaySoundatLocation 0 "/Game/CAS/Resource/Sound/sound_Hit.sound_Hit" "0, 0, 0" "0, 0, 0" 1.0 1.0 0.0 0 0 0 0)
          (return false))))))