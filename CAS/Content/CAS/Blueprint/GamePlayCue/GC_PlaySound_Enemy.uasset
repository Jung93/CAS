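; Gameplay cue that plays enemy combat sounds when executed on a target.
; OnExecute checks the target's Ability System Component tags in priority order (fire breath, taking damage, test attack, death) and plays only the first match's sound.
; Sounds play at the world origin rather than at the target's location, and matched branches return false.
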(fn OnExecute
  (params (MyTarget :type Actor%20Object%20Reference) (Parameters :type Gameplay%20Cue%20Parameters%20Structure%20%28by%20ref%29))
  (bind _returnvalue (Ability|GetAbilitySystemComponent MyTarget))
  (if (GameplayTags|HasMatchingGameplayTag _returnvalue "(TagName=\"Effect.Attack.FireBreath\")")
    (Audio|PlaySoundatLocation 0 "/Game/CAS/Resource/Sound/sound_FireBreath.sound_FireBreath" "0, 0, 0" "0, 0, 0" 1.0 1.0 0.0 0 0 0 0)
    (return false)
    (elif (GameplayTags|HasMatchingGameplayTag _returnvalue "(TagName=\"State.TakeDamage\")")
      (Audio|PlaySoundatLocation 0 "/Game/CAS/Resource/Sound/sound_Hit.sound_Hit" "0, 0, 0" "0, 0, 0" 1.0 1.0 0.0 0 0 0 0)
      (return false)
      (elif (GameplayTags|HasMatchingGameplayTag _returnvalue "(TagName=\"Effect.Attack.TEST\")")
        (Audio|PlaySoundatLocation 0 "/Game/CAS/Resource/Sound/sound_RoundKick.sound_RoundKick" "0, 0, 0" "0, 0, 0" 1.0 1.0 0.0 0 0 0 0)
        (return false)
        (elif (GameplayTags|HasMatchingGameplayTag _returnvalue "(TagName=\"State.Dead\")")
          (Audio|PlaySoundatLocation 0 "/Game/CAS/Resource/Sound/sound_Dead.sound_Dead" "0, 0, 0" "0, 0, 0" 1.0 1.0 0.0 0 0 0 0)
          (return false))))))