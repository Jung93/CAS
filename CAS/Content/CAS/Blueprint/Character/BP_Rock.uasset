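; BP_Rock is a rock actor that displays a key-press prompt when something enters its sensing area.
; On BeginPlay it creates a BP_KeyPressUI widget with an E-key texture and assigns it to a screen-space widget component.
; SenseCollider overlap events show the widget on entry and collapse it on exit, without filtering the overlapping actor.
; The file contains no key input handling.
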(event OnComponentBeginOverlap(SenseCollider)
  (params (OverlappedComponent :type Primitive%20Component%20Object%20Reference) (OtherActor :type Actor%20Object%20Reference) (OtherComp :type Primitive%20Component%20Object%20Reference) (OtherBodyIndex :type Integer) (bFromSweep :type Boolean) (SweepResult :type Hit%20Result%20Structure%20%28by%20ref%29))
  (Widget|SetVisibility (UserInterface|GetWidget (Variables|WidgetComponent|GetKeyPressWidgetComponent)) "Visible"))

(event OnComponentEndOverlap(SenseCollider)
  (params (OverlappedComponent :type Primitive%20Component%20Object%20Reference) (OtherActor :type Actor%20Object%20Reference) (OtherComp :type Primitive%20Component%20Object%20Reference) (OtherBodyIndex :type Integer))
  (Widget|SetVisibility (UserInterface|GetWidget (Variables|WidgetComponent|GetKeyPressWidgetComponent)) "Collapsed"))

(event EventBeginPlay
  (bind _keypresswidgetcomponent (Variables|WidgetComponent|GetKeyPressWidgetComponent))
  (bind _returnvalue (UserInterface|CreateWidget "/Game/CAS/Blueprint/UI/Interaction/BP_KeyPressUI.BP_KeyPressUI_C"))
  (Class|CASKeyPressUI|SetTexture _returnvalue "/Game/Assets/UI/Icon/T_e_128px_black.T_e_128px_black")
  (UserInterface|SetWidget _keypresswidgetcomponent _returnvalue)
  (Class|WidgetComponent|SetWidgetSpace _keypresswidgetcomponent "Screen"))

(event Collision|EventActorBeginOverlap
  (params (OtherActor :type Actor%20Object%20Reference)))

(event EventTick
  (params (DeltaSeconds :type Float%20%28single-precision%29)))

(fn ConstructionScript)